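; BP_HubWorldGameInstance is the hub world game instance Blueprint, holding hooks for a full-screen loading dialog.
; HideLoadingDialog removes the stored LoadingScreenWidget from its parent if it is valid.
; The RPG begin and end loading screen events are empty.
; A disconnected chain, which never runs, would create and show UI_FullScreenLoadingDialog a tick later on non-dedicated-server instances, so nothing here sets the widget.
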(event EventRPGBeginLoadingScreen)

(event EventRPGEndLoadingScreen)

(event EventHideLoadingDialog
  (bind _loadingscreenwidget (Variables|Default|GetLoadingScreenWidget))
  (Utilities|IsValid _loadingscreenwidget
    (:Is%20Valid
      (Widget|RemovefromParent _loadingscreenwidget))))